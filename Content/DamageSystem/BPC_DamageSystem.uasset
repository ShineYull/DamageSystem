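; Damage system component that tracks an owner's health, healing and death.
; TakeDamage runs a damage info struct through CanBeDamage, which branches to block, damage or no damage using dead, invincible and blocking state plus per-hit overrides.
; Damage clamps health and fires dispatchers for death or, when interruptible or forced, a damage response; blocked hits fire their own dispatcher.
; Heal restores clamped health only while alive.
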(fn `Heal`
  (params (InHealAmount :type "Float (double-precision)"))
  (returns (OutNewHealth :type "Float (double-precision)"))
  (if (not (`self.bIsDead`))
    (set `self.Health` (`KismetMathLibrary.FClamp` (+ (`self.Health`) (`local.InHealAmount`)) 0.0 (`self.MaxHealth`)))
    (return (`self.Health`))))

(fn `TakeDamage`
  (params (InDamageInfo :type "/Game/DamageSystem/S_DamageInfo Structure"))
  (returns (OutWasDamaged :type Boolean))
  (bind (_damageamount _damagetype _damageresponse _shoulddamageinvincible _canbeblocked) (break `/Game/DamageSystem/S_DamageInfo` (`local.InDamageInfo`)))
  (`self.CanBeDamage` _shoulddamageinvincible _canbeblocked
    (:`BlockDamage`
      (`self.Dispatcher_OnBlocked` (`.CanBeBlocked_19_74FDE7544DF92D8E36F092894FCA62B2` (break `/Game/DamageSystem/S_DamageInfo` (`local.InDamageInfo`))))
      (return false))
    (:`DoDamage`
      (set `self.Health` (`KismetMathLibrary.FClamp` (- (`self.Health`) (`.DamageAmount_4_954B38B84BAB20CEC60494BAD780819C` (break `/Game/DamageSystem/S_DamageInfo` (`local.InDamageInfo`)))) 0.0 (`self.MaxHealth`)))
      (if (<= (`self.Health`) 0.0)
        (set `self.bIsDead` true)
        (`self.Dispatcher_OnDeath`)
        (return true)
        (elif (or (`self.bIsInterruptible`) (`.ShouldForceInterrupt_22_20405340448FA5AC192752AE96B40BB4` (break `/Game/DamageSystem/S_DamageInfo` (`local.InDamageInfo`))))
          (`self.Dispatcher_OnDamageResponse` (`.DamageResponse_13_8DB3135944650BF0BCB90FBEC297CAFA` (break `/Game/DamageSystem/S_DamageInfo` (`local.InDamageInfo`))))
          (return true))))
    (:`NoDamage`
      (return false))))